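; Enemy AI pawn that chases a seen player and deals damage on reaching them.
; From both move start and success, delayed chains send it to an indexed target point, then clear the PawnSensing reference.
; A separate HitEnemy event, gated by a flag that CanHit sets, flings the mesh far upward with a rotation change over several seconds.
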(event OnSeePawn(PawnSensing)
  (params (Pawn :type Pawn%20Object%20Reference))
  (bind _asbp_player (Utilities|Casting|CastToBP_Player Pawn))
  (AI|AIMoveTo self "0, 0, 0" _asbp_player 5.0 false
    (:then
      _)
    (:OnSuccess
      (Game|Damage|ApplyDamage _asbp_player (Variables|Default|GetDamage) 0 self)))
  (Utilities|FlowControl|Delay 4.0)
  (AI|Navigation|SimpleMovetoActor (Pawn|GetController) (Utilities|Array|Get(acopy) (Variables|Default|GetTarget_Points) (Variables|Default|GetTarget_Point_Index)))
  (Utilities|FlowControl|Delay 3.0)
  (Variables|Default|SetPawnSensing 0))

(event Custom|HitEnemy
  (bind _mesh (Variables|Character|GetMesh))
  (if (stale Custom|CanHit _output_get)
    (Components|MoveComponentTo (Variables|Character|GetMesh) (+ (Variables|/Script/Engine.SceneComponent|GetRelativeLocation _mesh) "0, 0,6000.000000") (Math|Conversions|RotationFromXVector (+ (Math|Rotator|GetRotationXVector (Variables|/Script/Engine.SceneComponent|GetRelativeRotation _mesh)) "300.000000,400.000000,15000.000000")) false false 1e+01 false)))

(event Custom|CanHit
  (bind _output_get (Variables|Default|SetCanHitTrue? true)))

(fn ConstructionScript)